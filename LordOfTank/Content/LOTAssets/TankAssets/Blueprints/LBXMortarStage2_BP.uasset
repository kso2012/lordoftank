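; Second-stage mortar projectile that explodes with radial damage when it ends play.
; BeginPlay gives it a random forward speed in local space and a short random lifespan, so bursts vary in distance and timing.
; Hit destroys it only if the hit component equals its own class, so detonation effectively relies on lifespan expiry.
; EndPlay applies full damage in radius, ignoring all actors of this class, and spawns the explosion emitter and sound.
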(event `self.ReceiveBeginPlay`
  ;[1 0.1339 0.9812] Event Begin Play
  (`ProjectileMovementComponent.SetVelocityInLocalSpace` (`self.ProjectileMovement`) (`KismetMathLibrary.MakeVector` (`KismetMathLibrary.RandomFloatInRange` 1000.0 3000.0)))
  (`self.SetLifeSpan` (`KismetMathLibrary.RandomFloatInRange` 1.0 2.0)))

(event `self.ReceiveHit`
  (params (MyComp :type "PrimitiveComponent Object Reference") (Other :type "Actor Object Reference") (OtherComp :type "PrimitiveComponent Object Reference") (bSelfMoved :type Boolean) (HitLocation :type "Vector Structure") (HitNormal :type "Vector Structure") (NormalImpulse :type "Vector Structure") (Hit :type "HitResult Structure (by ref)"))
  ;[1 1 1] Event Hit
  (if (not (!= OtherComp "LBXMortarStage2_BP_C"))
    (`self.K2_DestroyActor`)))

(event `self.ReceiveEndPlay`
  (params (EndPlayReason :type "EEndPlayReason Enum" :default "Destroyed"))
  (bind _returnvalue (`self.K2_GetActorLocation`))
  ;[1 0.773 0] Event End Play
  (bind _outactors (`GameplayStatics.GetAllActorsOfClass` "LBXMortarStage2_BP_C"))
  (`GameplayStatics.ApplyRadialDamage` (`self.DamageDealt`) _returnvalue (`self.DamageRadius`) null _outactors null null true)
  (`GameplayStatics.SpawnEmitterAtLocation` (`self.ExplosionEmitter`) _returnvalue)
  (`GameplayStatics.PlaySoundAtLocation` (`self.ExplosionSound1`) _returnvalue))

(fn `UserConstructionScript`)