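; LBXMainProjectile_BP is the LBX main projectile in a tank game, exploding and dealing damage on impact.
; On hit it hides its mesh, applies damage, fires a radial force impulse, spawns explosion effects and sound, then destroys itself after a short delay.
; On EndPlay, if HUD crosshairs are hidden, it restores them and clears the player pawn's weapon follow-cam flag.
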(event `self.ReceiveHit`
  (params (MyComp :type "PrimitiveComponent Object Reference") (Other :type "Actor Object Reference") (OtherComp :type "PrimitiveComponent Object Reference") (bSelfMoved :type Boolean) (HitLocation :type "Vector Structure") (HitNormal :type "Vector Structure") (NormalImpulse :type "Vector Structure") (Hit :type "HitResult Structure (by ref)"))
  (bind (_bblockinghit _binitialoverlap _time _location _impactpoint _normal _impactnormal _physmat _hitactor) (`GameplayStatics.BreakHitResult` Hit))
  ;[1 1 1] Event Hit
  (`SceneComponent.SetVisibility` (`self.Projectile`) false false)
  (`GameplayStatics.ApplyDamage` _hitactor (`self.DamageDealt`) (`self.GetInstigatorController` (`self.Instigator`)) self)
  (`RadialForceComponent.FireImpulse` (`self.ExplosionForce`))
  (`GameplayStatics.SpawnEmitterAtLocation` (`self.ExplosionEmitter`) _impactpoint)
  (`GameplayStatics.PlaySoundAtLocation` (`self.ExplosionSound`) _impactpoint)
  (`KismetSystemLibrary.Delay` 0.5)
  (`self.K2_DestroyActor`))

(event `self.ReceiveEndPlay`
  (params (EndPlayReason :type "EEndPlayReason Enum" :default "Destroyed"))
  ;[1 0.773 0] Event End Play
  (bind _aslbxhud_bp (cast `/Game/LOTAssets/TankAssets/Blueprints/LBXHUD_BP` (`PlayerController.GetHUD` (`GameplayStatics.GetPlayerController` 0))))
  (if (!= (`/Game/LOTAssets/TankAssets/Blueprints/LBXHUD_BP.ShowCrosshairs` _aslbxhud_bp) true)
    (set `/Game/LOTAssets/TankAssets/Blueprints/LBXHUD_BP.ShowCrosshairs` true _aslbxhud_bp)
    (bind _aslbx1pawn_bp (cast `/Game/LOTAssets/TankAssets/Blueprints/LBX1Pawn_BP` (`GameplayStatics.GetPlayerPawn` 0)))
    (bind _lbxweapons (`/Game/LOTAssets/TankAssets/Blueprints/LBX1Pawn_BP.LBXWeapons` _aslbx1pawn_bp))
    (if (!= (`/Game/LOTAssets/TankAssets/Blueprints/Components/LBXWeapons.FollowCamActive?` _lbxweapons) false)
      (set `/Game/LOTAssets/TankAssets/Blueprints/Components/LBXWeapons.FollowCamActive?` false _lbxweapons))))

(fn `UserConstructionScript`)