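; Suspension component for the six-wheeled LBX1 pawn that springs its physics-simulated body off the ground.
; BeginPlay caches the body and wheel components and sets damping.
; While enabled, Tick sphere-traces down from each wheel socket, moves that wheel with a clamped height and applies normal-directed force that fades with hit distance.
; A body-center line trace adds double-strength spring force; only wheels 3–6 wire interpolation time and speed.
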(event `self.ReceiveBeginPlay`
  ;[1 0.1339 0.9812] Begin Play
  (bind _output_get (set `self.OwningPawn` (`self.GetOwner`)))
  (bind _aslbx1pawn_bp (cast `/Game/LOTAssets/TankAssets/Blueprints/LBX1Pawn_BP` _output_get))
  (`|ExecutionSequence`
    (:`then_0`
      (bind _output_get_2 (set `self.BodyMesh` (`/Game/LOTAssets/TankAssets/Blueprints/LBX1Pawn_BP.Body` _aslbx1pawn_bp)))
      (`PrimitiveComponent.SetSimulatePhysics` _output_get_2 true)
      (`PrimitiveComponent.SetLinearDamping` (`self.BodyMesh`) 1.0)
      (`PrimitiveComponent.SetAngularDamping` (`self.BodyMesh`) 0.6))
    (:`then_1`
      (set `self.Wheel1` (`/Game/LOTAssets/TankAssets/Blueprints/LBX1Pawn_BP.Wheel1` _aslbx1pawn_bp)))
    (:`then_2`
      (set `self.Wheel2` (`/Game/LOTAssets/TankAssets/Blueprints/LBX1Pawn_BP.Wheel2` _aslbx1pawn_bp)))
    (:`then_3`
      (set `self.Wheel3` (`/Game/LOTAssets/TankAssets/Blueprints/LBX1Pawn_BP.Wheel3` _aslbx1pawn_bp)))
    (:`then_4`
      (set `self.Wheel4` (`/Game/LOTAssets/TankAssets/Blueprints/LBX1Pawn_BP.Wheel4` _aslbx1pawn_bp)))
    (:`then_5`
      (set `self.Wheel5` (`/Game/LOTAssets/TankAssets/Blueprints/LBX1Pawn_BP.Wheel5` _aslbx1pawn_bp)))
    (:`then_6`
      (set `self.Wheel6` (`/Game/LOTAssets/TankAssets/Blueprints/LBX1Pawn_BP.Wheel6` _aslbx1pawn_bp)))))

(event `BodySuspensionMovement`
  (bind _returnvalue (`SceneComponent.K2_GetComponentLocation` (`self.BodyMesh`)))
  (bind _returnvalue_2 (`SceneComponent.K2_GetComponentLocation` (`self.BodyMesh`)))
  ;[1 0.773 0] Body Suspension
  (bind (_outhit _returnvalue_3) (`KismetSystemLibrary.LineTraceSingle` _returnvalue_2 (- _returnvalue_2 (`KismetMathLibrary.MakeVector` 0.0 0.0 (`self.TraceLength`))) "TraceTypeQuery1" false (`|MakeArray` (`self.OwningPawn`)) (`self.DebugTraceLines`)))
  (if _returnvalue_3
    (bind (_bblockinghit _binitialoverlap _time _location _impactpoint _normal _impactnormal) (`GameplayStatics.BreakHitResult` _outhit))
    (`PrimitiveComponent.AddForceAtLocation` (`self.BodyMesh`) (* _impactnormal (`KismetMathLibrary.Lerp` (* (`self.SpringForce`) 2.0) 0.0 (/ (`KismetMathLibrary.VSize` (- _impactpoint _returnvalue)) (`self.TraceLength`)))) _returnvalue "None")))

(event `self.ReceiveTick`
  (params (DeltaSeconds :type "Float (single-precision)"))
  ;[1 1 1] Event Tick
  (if (`self.EnableSuspension?`)
    (`self.Wheel1Movement`)
    (`self.Wheel2Movement`)
    (`self.Wheel3Movement`)
    (`self.Wheel4Movement`)
    (`self.Wheel5Movement`)
    (`self.Wheel6Movement`)
    (`self.BodySuspensionMovement`)))

(event `Wheel1Movement`
  (bind _maxwheelmovement (`self.MaxWheelMovement`))
  (bind _returnvalue (`SceneComponent.GetSocketLocation` (`self.BodyMesh`) "Wheel1"))
  (bind _returnvalue_2 (`SceneComponent.GetSocketLocation` (`self.BodyMesh`) "Wheel1"))
  (bind (_relativelocation_x _relativelocation_y _relativelocation_z) (`KismetMathLibrary.BreakVector` (`SceneComponent.RelativeLocation` (`self.Wheel1`))))
  ;[0 1 0.1843] Wheel1
  (bind _outhit (`KismetSystemLibrary.SphereTraceSingle_NEW` _returnvalue (- _returnvalue (`KismetMathLibrary.MakeVector` 0.0 0.0 (`self.TraceLength`))) (`self.SphereTraceRadius`) "TraceTypeQuery1" false (`|MakeArray` (`self.OwningPawn`)) (`self.DebugTraceLines`)))
  (bind (_bblockinghit _binitialoverlap _time _location _impactpoint _normal _impactnormal) (`GameplayStatics.BreakHitResult` _outhit))
  (bind _returnvalue_3 (- _impactpoint _returnvalue_2))
  (bind (_returnvalue_x _returnvalue_y _returnvalue_z) (`KismetMathLibrary.BreakVector` (`KismetMathLibrary.VInterpTo` _returnvalue_2 (`KismetMathLibrary.MakeVector` 0.0 0.0 (+ (.z _returnvalue_3) (`self.WheelRadius`))))))
  (`SceneComponent.K2_SetRelativeLocation` (`self.Wheel1`) (`KismetMathLibrary.MakeVector` 0.0 0.0 _returnvalue_z) false false)
  (`PrimitiveComponent.AddForceAtLocation` (`self.BodyMesh`) (* _impactnormal (`KismetMathLibrary.Lerp` (`self.SpringForce`) 0.0 (/ (`KismetMathLibrary.VSize` _returnvalue_3) (`self.TraceLength`)))) (`SceneComponent.GetSocketLocation` (`self.BodyMesh`) "Wheel1") "Wheel1")
  (`SceneComponent.K2_SetRelativeLocation` (`self.Wheel1`) (`KismetMathLibrary.MakeVector` 0.0 0.0 (`KismetMathLibrary.FClamp` _relativelocation_z (* _maxwheelmovement -1.0) _maxwheelmovement)) false false))

(event `Wheel2Movement`
  (bind _maxwheelmovement (`self.MaxWheelMovement`))
  (bind _returnvalue (`SceneComponent.GetSocketLocation` (`self.BodyMesh`) "Wheel2"))
  (bind _returnvalue_2 (`SceneComponent.GetSocketLocation` (`self.BodyMesh`) "Wheel2"))
  (bind (_relativelocation_x _relativelocation_y _relativelocation_z) (`KismetMathLibrary.BreakVector` (`SceneComponent.RelativeLocation` (`self.Wheel2`))))
  ;[1 1 1] Wheel2
  (bind _outhit (`KismetSystemLibrary.SphereTraceSingle_NEW` _returnvalue (- _returnvalue (`KismetMathLibrary.MakeVector` 0.0 0.0 (`self.TraceLength`))) (`self.SphereTraceRadius`) "TraceTypeQuery1" false (`|MakeArray` (`self.OwningPawn`)) (`self.DebugTraceLines`)))
  (bind (_bblockinghit _binitialoverlap _time _location _impactpoint _normal _impactnormal) (`GameplayStatics.BreakHitResult` _outhit))
  (bind _returnvalue_3 (- _impactpoint _returnvalue_2))
  (bind (_returnvalue_x _returnvalue_y _returnvalue_z) (`KismetMathLibrary.BreakVector` (`KismetMathLibrary.VInterpTo` _returnvalue_2 (`KismetMathLibrary.MakeVector` 0.0 0.0 (+ (.z _returnvalue_3) (`self.WheelRadius`))))))
  (`SceneComponent.K2_SetRelativeLocation` (`self.Wheel2`) (`KismetMathLibrary.MakeVector` 0.0 0.0 _returnvalue_z) false false)
  (`PrimitiveComponent.AddForceAtLocation` (`self.BodyMesh`) (* _impactnormal (`KismetMathLibrary.Lerp` (`self.SpringForce`) 0.0 (/ (`KismetMathLibrary.VSize` _returnvalue_3) (`self.TraceLength`)))) (`SceneComponent.GetSocketLocation` (`self.BodyMesh`) "Wheel2") "Wheel2")
  (`SceneComponent.K2_SetRelativeLocation` (`self.Wheel2`) (`KismetMathLibrary.MakeVector` 0.0 0.0 (`KismetMathLibrary.FClamp` _relativelocation_z (* _maxwheelmovement -1.0) _maxwheelmovement)) false false))

(event `Wheel3Movement`
  (bind _maxwheelmovement (`self.MaxWheelMovement`))
  (bind _returnvalue (`SceneComponent.GetSocketLocation` (`self.BodyMesh`) "Wheel3"))
  (bind _returnvalue_2 (`SceneComponent.GetSocketLocation` (`self.BodyMesh`) "Wheel3"))
  (bind (_relativelocation_x _relativelocation_y _relativelocation_z) (`KismetMathLibrary.BreakVector` (`SceneComponent.RelativeLocation` (`self.Wheel3`))))
  ;[0 1 0.1843] Wheel 3
  (bind _outhit (`KismetSystemLibrary.SphereTraceSingle_NEW` _returnvalue (- _returnvalue (`KismetMathLibrary.MakeVector` 0.0 0.0 (`self.TraceLength`))) (`self.SphereTraceRadius`) "TraceTypeQuery1" false (`|MakeArray` (`self.OwningPawn`)) (`self.DebugTraceLines`)))
  (bind (_bblockinghit _binitialoverlap _time _location _impactpoint _normal _impactnormal) (`GameplayStatics.BreakHitResult` _outhit))
  (bind _returnvalue_3 (- _impactpoint _returnvalue_2))
  (bind (_returnvalue_x _returnvalue_y _returnvalue_z) (`KismetMathLibrary.BreakVector` (`KismetMathLibrary.VInterpTo` _returnvalue_2 (`KismetMathLibrary.MakeVector` 0.0 0.0 (+ (.z _returnvalue_3) (`self.WheelRadius`))) (`GameplayStatics.GetWorldDeltaSeconds`) (`self.InterpSpeed`))))
  (`SceneComponent.K2_SetRelativeLocation` (`self.Wheel3`) (`KismetMathLibrary.MakeVector` 0.0 0.0 _returnvalue_z) false false)
  (`PrimitiveComponent.AddForceAtLocation` (`self.BodyMesh`) (* _impactnormal (`KismetMathLibrary.Lerp` (`self.SpringForce`) 0.0 (/ (`KismetMathLibrary.VSize` _returnvalue_3) (`self.TraceLength`)))) (`SceneComponent.GetSocketLocation` (`self.BodyMesh`) "Wheel3") "Wheel3")
  (`SceneComponent.K2_SetRelativeLocation` (`self.Wheel3`) (`KismetMathLibrary.MakeVector` 0.0 0.0 (`KismetMathLibrary.FClamp` _relativelocation_z (* _maxwheelmovement -1.0) _maxwheelmovement)) false false))

(event `Wheel4Movement`
  (bind _maxwheelmovement (`self.MaxWheelMovement`))
  (bind _returnvalue (`SceneComponent.GetSocketLocation` (`self.BodyMesh`) "Wheel4"))
  (bind _returnvalue_2 (`SceneComponent.GetSocketLocation` (`self.BodyMesh`) "Wheel4"))
  (bind (_relativelocation_x _relativelocation_y _relativelocation_z) (`KismetMathLibrary.BreakVector` (`SceneComponent.RelativeLocation` (`self.Wheel4`))))
  ;[1 1 1] Wheel 4
  (bind _outhit (`KismetSystemLibrary.SphereTraceSingle_NEW` _returnvalue (- _returnvalue (`KismetMathLibrary.MakeVector` 0.0 0.0 (`self.TraceLength`))) (`self.SphereTraceRadius`) "TraceTypeQuery1" false (`|MakeArray` (`self.OwningPawn`)) (`self.DebugTraceLines`)))
  (bind (_bblockinghit _binitialoverlap _time _location _impactpoint _normal _impactnormal) (`GameplayStatics.BreakHitResult` _outhit))
  (bind _returnvalue_3 (- _impactpoint _returnvalue_2))
  (bind (_returnvalue_x _returnvalue_y _returnvalue_z) (`KismetMathLibrary.BreakVector` (`KismetMathLibrary.VInterpTo` _returnvalue_2 (`KismetMathLibrary.MakeVector` 0.0 0.0 (+ (.z _returnvalue_3) (`self.WheelRadius`))) (`GameplayStatics.GetWorldDeltaSeconds`) (`self.InterpSpeed`))))
  (`SceneComponent.K2_SetRelativeLocation` (`self.Wheel4`) (`KismetMathLibrary.MakeVector` 0.0 0.0 _returnvalue_z) false false)
  (`PrimitiveComponent.AddForceAtLocation` (`self.BodyMesh`) (* _impactnormal (`KismetMathLibrary.Lerp` (`self.SpringForce`) 0.0 (/ (`KismetMathLibrary.VSize` _returnvalue_3) (`self.TraceLength`)))) (`SceneComponent.GetSocketLocation` (`self.BodyMesh`) "Wheel4") "Wheel4")
  (`SceneComponent.K2_SetRelativeLocation` (`self.Wheel4`) (`KismetMathLibrary.MakeVector` 0.0 0.0 (`KismetMathLibrary.FClamp` _relativelocation_z (* _maxwheelmovement -1.0) _maxwheelmovement)) false false))

(event `Wheel5Movement`
  (bind _maxwheelmovement (`self.MaxWheelMovement`))
  (bind _returnvalue (`SceneComponent.GetSocketLocation` (`self.BodyMesh`) "Wheel5"))
  (bind _returnvalue_2 (`SceneComponent.GetSocketLocation` (`self.BodyMesh`) "Wheel5"))
  (bind (_relativelocation_x _relativelocation_y _relativelocation_z) (`KismetMathLibrary.BreakVector` (`SceneComponent.RelativeLocation` (`self.Wheel5`))))
  ;[0 1 0.1843] Wheel 5
  (bind _outhit (`KismetSystemLibrary.SphereTraceSingle_NEW` _returnvalue (- _returnvalue (`KismetMathLibrary.MakeVector` 0.0 0.0 (`self.TraceLength`))) (`self.SphereTraceRadius`) "TraceTypeQuery1" false (`|MakeArray` (`self.OwningPawn`)) (`self.DebugTraceLines`)))
  (bind (_bblockinghit _binitialoverlap _time _location _impactpoint _normal _impactnormal) (`GameplayStatics.BreakHitResult` _outhit))
  (bind _returnvalue_3 (- _impactpoint _returnvalue_2))
  (bind (_returnvalue_x _returnvalue_y _returnvalue_z) (`KismetMathLibrary.BreakVector` (`KismetMathLibrary.VInterpTo` _returnvalue_2 (`KismetMathLibrary.MakeVector` 0.0 0.0 (+ (.z _returnvalue_3) (`self.WheelRadius`))) (`GameplayStatics.GetWorldDeltaSeconds`) (`self.InterpSpeed`))))
  (`SceneComponent.K2_SetRelativeLocation` (`self.Wheel5`) (`KismetMathLibrary.MakeVector` 0.0 0.0 _returnvalue_z) false false)
  (`PrimitiveComponent.AddForceAtLocation` (`self.BodyMesh`) (* _impactnormal (`KismetMathLibrary.Lerp` (`self.SpringForce`) 0.0 (/ (`KismetMathLibrary.VSize` _returnvalue_3) (`self.TraceLength`)))) (`SceneComponent.GetSocketLocation` (`self.BodyMesh`) "Wheel5") "Wheel5")
  (`SceneComponent.K2_SetRelativeLocation` (`self.Wheel5`) (`KismetMathLibrary.MakeVector` 0.0 0.0 (`KismetMathLibrary.FClamp` _relativelocation_z (* _maxwheelmovement -1.0) _maxwheelmovement)) false false))

(event `Wheel6Movement`
  (bind _maxwheelmovement (`self.MaxWheelMovement`))
  (bind _returnvalue (`SceneComponent.GetSocketLocation` (`self.BodyMesh`) "Wheel6"))
  (bind _returnvalue_2 (`SceneComponent.GetSocketLocation` (`self.BodyMesh`) "Wheel6"))
  (bind (_relativelocation_x _relativelocation_y _relativelocation_z) (`KismetMathLibrary.BreakVector` (`SceneComponent.RelativeLocation` (`self.Wheel6`))))
  ;[1 1 1] Wheel 6
  (bind _outhit (`KismetSystemLibrary.SphereTraceSingle_NEW` _returnvalue (- _returnvalue (`KismetMathLibrary.MakeVector` 0.0 0.0 (`self.TraceLength`))) (`self.SphereTraceRadius`) "TraceTypeQuery1" false (`|MakeArray` (`self.OwningPawn`)) (`self.DebugTraceLines`)))
  (bind (_bblockinghit _binitialoverlap _time _location _impactpoint _normal _impactnormal) (`GameplayStatics.BreakHitResult` _outhit))
  (bind _returnvalue_3 (- _impactpoint _returnvalue_2))
  (bind (_returnvalue_x _returnvalue_y _returnvalue_z) (`KismetMathLibrary.BreakVector` (`KismetMathLibrary.VInterpTo` _returnvalue_2 (`KismetMathLibrary.MakeVector` 0.0 0.0 (+ (.z _returnvalue_3) (`self.WheelRadius`))) (`GameplayStatics.GetWorldDeltaSeconds`) (`self.InterpSpeed`))))
  (`SceneComponent.K2_SetRelativeLocation` (`self.Wheel6`) (`KismetMathLibrary.MakeVector` 0.0 0.0 _returnvalue_z) false false)
  (`PrimitiveComponent.AddForceAtLocation` (`self.BodyMesh`) (* _impactnormal (`KismetMathLibrary.Lerp` (`self.SpringForce`) 0.0 (/ (`KismetMathLibrary.VSize` _returnvalue_3) (`self.TraceLength`)))) (`SceneComponent.GetSocketLocation` (`self.BodyMesh`) "Wheel6") "Wheel6")
  (`SceneComponent.K2_SetRelativeLocation` (`self.Wheel6`) (`KismetMathLibrary.MakeVector` 0.0 0.0 (`KismetMathLibrary.FClamp` _relativelocation_z (* _maxwheelmovement -1.0) _maxwheelmovement)) false false))