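; Movement component for a tank pawn that handles driving, turning, turret yaw and barrel pitch.
; Axis handler events offset and rotate the owning pawn with delta-time scaling, spinning wheel meshes cosmetically, with left and right sets counter-rotating on turns.
; Turret and barrel handlers add rate-scaled local rotation per call, without delta time.
; Tick subtracts the stored axis values from turret yaw and barrel pitch, then clamps both to their limits.
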(event `self.ReceiveBeginPlay`
  ;[1 0.1339 0.9812] Event Begin Play
  (`|ExecutionSequence`
    (:`then_0`
      (bind _aspawn (cast `Pawn` (`self.GetOwner`)))
      (set `self.Owner Pawn` _aspawn))))

(event `ForwardMovementHandler`
  (params (`Forward Axis Value` :type "Float (double-precision)"))
  (bind _forwardaxisvalue (`self.ForwardAxisValue`))
  ;[0 1 0] Forward Movement
  (set `self.ForwardAxisValue` `Forward Axis Value`)
  (`Actor.K2_AddActorLocalOffset` (`self.Owner Pawn`) (`KismetMathLibrary.MakeVector` (* (`GameplayStatics.GetWorldDeltaSeconds`) (* (`self.ForwardAxisValue`) (`self.VehicleMaxSpeed`)))) false false)
  (for _array_element (`self.AllWheels`)
    (`SceneComponent.K2_AddLocalRotation` _array_element (`KismetMathLibrary.MakeRotator` 0.0 (* (`KismetMathLibrary.SelectFloat` 1.0 -1.0 (> _forwardaxisvalue 1.0)) (* _forwardaxisvalue (/ (`self.VehicleMaxSpeed`) 100.0)))) false false)))

(event `TurningMovementHandler`
  (params (`Turn Axis Value` :type "Float (double-precision)"))
  (bind _turnaxisvalue (`self.TurnAxisValue`))
  (bind _turnaxisvalue_2 (`self.TurnAxisValue`))
  ;[0 1 0] Turning Movement
  (set `self.TurnAxisValue` `Turn Axis Value`)
  (`Actor.K2_AddActorLocalRotation` (`self.Owner Pawn`) (`KismetMathLibrary.MakeRotator` 0.0 0.0 (* (`GameplayStatics.GetWorldDeltaSeconds`) (* (`self.TurnAxisValue`) (`self.VehicleTurnRate`)))) false false)
  (`|ExecutionSequence`
    (:`then_0`
      (for _array_element (`self.RightWheels`)
        (`SceneComponent.K2_AddLocalRotation` _array_element (`KismetMathLibrary.MakeRotator` 0.0 (* (`KismetMathLibrary.SelectFloat` -1.0 1.0 (> _turnaxisvalue 1.0)) (* _turnaxisvalue (/ (/ (`self.VehicleMaxSpeed`) 100.0) 1.66)))) false false)))
    (:`then_1`
      (for _array_element_2 (`self.LeftWheels`)
        (`SceneComponent.K2_AddLocalRotation` _array_element_2 (`KismetMathLibrary.MakeRotator` 0.0 (* (`KismetMathLibrary.SelectFloat` 1.0 -1.0 (> _turnaxisvalue_2 1.0)) (* _turnaxisvalue_2 (/ (/ (`self.VehicleMaxSpeed`) 100.0) 1.6666)))) false false)))))

(event `BarrelMovementHandler`
  (params (AxisValue :type "Float (double-precision)"))
  ;[0 0 1] Barrel Movement
  (set `self.BarrelAxisValue` AxisValue)
  (`SceneComponent.K2_AddLocalRotation` (`self.BarrelMesh`) (`KismetMathLibrary.MakeRotator` 0.0 (* (`self.BarrelAxisValue`) (`self.BarrelPitchRate`))) false false))

(event `TurretMovementHandler`
  (params (AxisValue :type "Float (double-precision)"))
  ;[0 0 1] Turret Movement
  (set `self.TurretAxisValue` AxisValue)
  (`SceneComponent.K2_AddLocalRotation` (`self.TurretMesh`) (`KismetMathLibrary.MakeRotator` 0.0 0.0 (* (`self.TurretAxisValue`) (`self.TurretTurnRate`))) false false))

(event `self.ReceiveTick`
  (params (DeltaSeconds :type "Float (single-precision)"))
  (bind _turretdegreeclamp (`self.TurretDegreeClamp`))
  ;[1 1 1] Event Tick
  ;[0.03979 1 0.9809] Turret Movement Clamping
  (`SceneComponent.K2_SetRelativeRotation` (`self.TurretMesh`) (`KismetMathLibrary.MakeRotator` 0.0 0.0 (`KismetMathLibrary.FClamp` (+ (* (`self.TurretAxisValue`) -1.0) (.yaw (`SceneComponent.RelativeRotation` (`self.TurretMesh`)))) (* _turretdegreeclamp -1.0) _turretdegreeclamp)) false false)
  ;[0.03979 1 0.9809] Barrel Movement Clamping
  (`SceneComponent.K2_SetRelativeRotation` (`self.BarrelMesh`) (`KismetMathLibrary.MakeRotator` 0.0 (`KismetMathLibrary.FClamp` (+ (* (`self.BarrelAxisValue`) -1.0) (.pitch (`SceneComponent.RelativeRotation` (`self.BarrelMesh`)))) -5.0 30.0)) false false))