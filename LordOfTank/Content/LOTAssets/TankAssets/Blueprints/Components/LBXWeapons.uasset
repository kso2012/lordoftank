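; Weapons component for the LBX tank pawn that fires cannon and mortar rounds, with cooldowns and a timed reload.
; A camera-center trace aims projectiles spawned at the barrel muzzle, with sound, shake and smoke.
; A gated retriggerable-delay loop advances reload progress.
; Holding fire half a second after a shot hides crosshairs and blends the view to the round, found by PlayerId tag, blocking further firing while active.
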(event `self.ReceiveBeginPlay`
  ;[1 0.1339 0.9812] Begin Play
  (bind _aslbx1pawn_bp (cast `/Game/LOTAssets/TankAssets/Blueprints/LBX1Pawn_BP` (`self.GetOwner`)))
  (set `self.Owner Pawn` _aslbx1pawn_bp)
  (set `self.ProjectileTag` (`KismetStringLibrary.Conv_StringToName` (`KismetStringLibrary.Conv_DoubleToString` (`/Game/LOTAssets/TankAssets/Blueprints/LBX1Pawn_BP.RandomProjectileTag` _aslbx1pawn_bp)))))

(event `FireWeapon`
  (bind _currentprojectile (`self.CurrentProjectile`))
  (bind _owner_pawn (`self.Owner Pawn`))
  (bind _returnvalue_location (`KismetMathLibrary.BreakTransform` (`SceneComponent.GetSocketTransform` (`self.BarrelMesh`) "Muzzle" "RTS_World")))
  (bind _returnvalue (`SceneComponent.GetSocketTransform` (`self.BarrelMesh`) "Muzzle" "RTS_World"))
  (bind _transformcomponent (`PlayerCameraManager.TransformComponent` (`GameplayStatics.GetPlayerCameraManager` 0)))
  (bind _returnvalue_2 (`SceneComponent.K2_GetComponentLocation` _transformcomponent))
  (bind _returnvalue_3 (+ _returnvalue_2 (* (`SceneComponent.GetForwardVector` _transformcomponent) 500000.0)))
  (bind _array (`|MakeArray` (`KismetStringLibrary.Conv_StringToName` (`KismetStringLibrary.Conv_IntToString` (`PlayerState.PlayerId` (`Controller.PlayerState` (`GameplayStatics.GetPlayerController` 0)))))))
  ;[1 0 0] Fire Weapon
  (set `self.MaxAccuracyRange` _returnvalue_3)
  (bind (_outhit _returnvalue_4) (`KismetSystemLibrary.LineTraceSingle` _returnvalue_2 _returnvalue_3 "TraceTypeQuery1" true))
  (if _returnvalue_4
    (bind _returnvalue_5 (`|SpawnActorFromClass` _currentprojectile (`KismetMathLibrary.MakeTransform` _returnvalue_location (`KismetMathLibrary.MakeRotFromX` (- (`.ImpactPoint` (`GameplayStatics.BreakHitResult` _outhit)) _returnvalue_location))) "Undefined" "OverrideRootScale" null _owner_pawn))
    (set `Actor.Tags` _array _returnvalue_5)
    (else
      (bind _returnvalue_6 (`|SpawnActorFromClass` _currentprojectile (`KismetMathLibrary.MakeTransform` _returnvalue_location (`KismetMathLibrary.MakeRotFromX` (- (`self.MaxAccuracyRange`) _returnvalue_location))) "Undefined" "OverrideRootScale" null _owner_pawn))
      (set `Actor.Tags` _array _returnvalue_6)))
  (set `self.MuzzleLocation` (.location _returnvalue))
  (`GameplayStatics.SpawnSoundAtLocation` "/Game/TankAsset/Audio/Explosion02.Explosion02" (`self.MuzzleLocation`))
  (`GameplayStatics.PlayWorldCameraShake` "/Game/LOTAssets/TankAssets/Blueprints/LBXCannonCameraShake_BP.LBXCannonCameraShake_BP_C" (`self.MuzzleLocation`) 0.0 4000.0)
  (`GameplayStatics.SpawnEmitterAtLocation` "/Game/LOTAssets/TankAssets/Particles/PT_MuzzleSmoke.PT_MuzzleSmoke" (`self.MuzzleLocation`) (.rotation _returnvalue)))

(event `ReloadWeapon`
  (bind _reloadtimecurrent (`self.ReloadTimeCurrent`))
  ;[0.03979 1 0.9809] Reload Weapon
  (set `self.ReloadTimeCurrent` 0.0)
  (set `self.ReloadComplete?` false)
  (`|ExecutionSequence`
    (:`then_0`
      (goto _label :!via `Open`))
    (:`then_1`
      (`/Engine/EditorBlueprintResources/StandardMacros.Gate` true :!label _label
        (:`Exit`
          (if (>= _reloadtimecurrent (`self.ReloadTimeMax`))
            (set `self.ReloadComplete?` true)
            (else
              (set `self.ReloadTimeCurrent` (+ _reloadtimecurrent 0.1))
              (`KismetSystemLibrary.RetriggerableDelay` 0.1)
              (if (`self.ReloadComplete?`)
                (set `self.ReloadTimeCurrent` 1.0)
                (goto _label :!via `Close`)
                (else
                  (goto _label))))))))))

(event `FireMainCannon`
  (bind _returnvalue (`GameplayStatics.GetPlayerController` 0))
  ;[1 0 0] Cannon Fire Function
  (set `self.CurrentProjectile` (`self.CannonProjectile`))
  (if (and (`self.CannonReadyToFire?`) (`self.ReloadComplete?`) (!= (`self.FollowCamActive?`) true))
    (set `self.ReloadTimeMax` (`self.CannonCoolDownTime`))
    (set `self.CannonReadyToFire?` false)
    (`self.ReloadWeapon`)
    (`|ExecutionSequence`
      (:`then_0`
        (`self.FireWeapon`)
        (`KismetSystemLibrary.Delay` (`self.CannonCoolDownTime`))
        (set `self.CannonReadyToFire?` true)
        (set `self.Recoil?` true))
      (:`then_1`
        (`KismetSystemLibrary.Delay` 0.5)
        (if (or (`PlayerController.IsInputKeyDown` _returnvalue "Gamepad_RightTrigger") (`PlayerController.IsInputKeyDown` _returnvalue "LeftMouseButton"))
          (`self.FollowRound`))))))

(event `FireMortar`
  (bind _returnvalue (`GameplayStatics.GetPlayerController` 0))
  ;[1 0 0] Mortar Fire Function
  (set `self.CurrentProjectile` (`self.MortarProjectile`))
  (if (and (`self.MortarReadyToFire?`) (`self.ReloadComplete?`) (!= (`self.FollowCamActive?`) true))
    (set `self.ReloadTimeMax` (`self.MortarCoolDownTime`))
    (set `self.MortarReadyToFire?` false)
    (`self.ReloadWeapon`)
    (`|ExecutionSequence`
      (:`then_0`
        (`self.FireWeapon`)
        (`KismetSystemLibrary.Delay` (`self.MortarCoolDownTime`))
        (set `self.MortarReadyToFire?` true)
        (set `self.Recoil?` true))
      (:`then_1`
        (`KismetSystemLibrary.Delay` 0.5)
        (if (or (`PlayerController.IsInputKeyDown` _returnvalue "Gamepad_RightTrigger") (`PlayerController.IsInputKeyDown` _returnvalue "LeftMouseButton"))
          (`self.FollowRound`))))))

(event `FollowRound`
  (bind _returnvalue (`GameplayStatics.GetPlayerController` 0))
  ;[1 0.773 0] Follow Round Fired - Follow Cam
  (bind _outactors (`GameplayStatics.GetAllActorsOfClass` (`self.CurrentProjectile`)))
  (for (_array_element _array_index) _outactors
    (if (`Actor.ActorHasTag` _array_element (`KismetStringLibrary.Conv_StringToName` (`KismetStringLibrary.Conv_IntToString` (`PlayerState.PlayerId` (`Controller.PlayerState` (`GameplayStatics.GetPlayerController` 0))))))
      (if (== (`KismetArrayLibrary.Array_LastIndex` _outactors) _array_index)
        (bind _aslbxhud_bp (cast `/Game/LOTAssets/TankAssets/Blueprints/LBXHUD_BP` (`PlayerController.GetHUD` _returnvalue)))
        (set `/Game/LOTAssets/TankAssets/Blueprints/LBXHUD_BP.ShowCrosshairs` false _aslbxhud_bp)
        (`PlayerController.SetViewTargetWithBlend` _returnvalue _array_element 0.5 "VTBlend_Linear" 0.0 false)
        (set `self.FollowCamActive?` true)))))