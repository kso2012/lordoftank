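; Aiming component for the LBX1 tank pawn that previews the mortar's ballistic arc while the turret camera is active.
; Once activated, each tick it samples the trajectory from the barrel muzzle using the projectile class's initial velocity and world gravity.
; It line-traces each time segment, draws every Nth as a debug line, and places a surface-aligned decal on hits.
; A debug flag adds printouts and a test arrow.
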(event `self.ReceiveBeginPlay`
  ;[1 0.1339 0.9812] Event Begin Play
  (bind _aslbx1pawn_bp (cast `/Game/LOTAssets/TankAssets/Blueprints/LBX1Pawn_BP` (`self.GetOwner`))
    (:`then`
      (set `self.OwningPawn` _aslbx1pawn_bp)
      (bind _outactors (`GameplayStatics.GetAllActorsOfClass` "/Script/Engine.WorldSettings"))
      (bind _globalgravityz (`WorldSettings.GlobalGravityZ` (`KismetArrayLibrary.Array_Get` _outactors)))
      (set `self.WorldSettingsGravity` (`KismetMathLibrary.MakeVector` 0.0 0.0 _globalgravityz))
      (`KismetSystemLibrary.Delay` 0.5)
      (if (`self.DebuggingArcs?`)
        (`KismetSystemLibrary.PrintString` (`KismetStringLibrary.Concat_StrStr` "World Settings - Global Gravity Z Settings: " (`KismetStringLibrary.Conv_DoubleToString` _globalgravityz)) true true (struct :`G` 0.66 :`B` 1.0 :`A` 1.0) 10.0)))
    (:`CastFailed`
      (`KismetSystemLibrary.PrintString` "Failed to get owner LBX1"))))

(event `DrawArcPath`
  ;[1 0.773 0] Draw Arc Path
  (set `self.DrawArcActivated?` true))

(event `self.ReceiveTick`
  (params (DeltaSeconds :type "Float (single-precision)"))
  (bind _owningpawn (`self.OwningPawn`))
  (bind _barrel (`/Game/LOTAssets/TankAssets/Blueprints/LBX1Pawn_BP.Barrel` _owningpawn))
  (bind _returnvalue_location (`KismetMathLibrary.BreakTransform` (`SceneComponent.GetSocketTransform` _barrel "Muzzle" "RTS_World")))
  ;[1 1 1] Event Tick
  (`self.RenderDecal` false)
  (`SceneComponent.SetVisibility` (`self.TestingArrow`) false false)
  (if (`self.DrawArcActivated?`)
    (if (`/Game/LOTAssets/TankAssets/Blueprints/LBX1Pawn_BP.TurretCamActive?` _owningpawn)
      (bind _aslbxmortar_stage_1_bp (castclass `/Game/LOTAssets/TankAssets/Blueprints/LBXMortarStage1_BP` (`/Game/LOTAssets/TankAssets/Blueprints/Components/LBXWeapons.CurrentProjectile` (`/Game/LOTAssets/TankAssets/Blueprints/LBX1Pawn_BP.LBXWeapons` _owningpawn)))
        (:`then`
          (set `self.ProjectileVelocity` (`.InitialVelocity` (defaults `/Game/LOTAssets/TankAssets/Blueprints/Components/LBXArcAiming` _aslbxmortar_stage_1_bp)))
          (set `self.MuzzleLocation` _returnvalue_location)
          (set `self.InitialVelocity` (`KismetMathLibrary.TransformDirection` (`SceneComponent.GetSocketTransform` _barrel "Muzzle" "RTS_World") (`self.ProjectileVelocity`)))
          (for _index (range (+ (`KismetMathLibrary.FFloor` (/ (`self.PathLifeTime`) (`self.TimeInterval`))) 1)) :!label _label
            (bind (_point1 _point2) (`self.GetArcSegmentAtTime` (`self.MuzzleLocation`) (`self.InitialVelocity`) (`self.WorldSettingsGravity`) (* _index (`self.TimeInterval`)) (* (+ _index 1) (`self.TimeInterval`))))
            (bind (_outhit _returnvalue) (`KismetSystemLibrary.LineTraceSingle` _point1 _point2 "TraceTypeQuery1" true (`|MakeArray` (`self.OwningPawn`) :!type "Actor Object Reference")))
            (`self.RenderArcSegment` _point1 _point2 (`self.ArcDrawType`) _index)
            (if _returnvalue
              (`self.RenderDecal` true)
              (bind (_bblockinghit _binitialoverlap _time _location _impactpoint _normal _impactnormal _physmat _hitactor) (`GameplayStatics.BreakHitResult` _outhit))
              (`SceneComponent.K2_SetWorldLocationAndRotation` (`self.ArcDecal`) _impactpoint (`KismetMathLibrary.MakeRotFromX` _impactnormal) false false)
              (if (`self.DebuggingArcs?`)
                (`KismetSystemLibrary.PrintString` (`KismetStringLibrary.Concat_StrStr` "HIt: " (`KismetSystemLibrary.GetDisplayName` _hitactor)) true true (struct :`G` 0.66 :`B` 1.0 :`A` 1.0) 0.5)
                (`SceneComponent.SetVisibility` (`self.TestingArrow`) true false)))))
        (:`CastFailed`
          (`KismetSystemLibrary.PrintString` "Failed cast to mortar"))))))

(event `BreakArcPathDraw`
  ;[1 0.773 0] Break Arc Path Draw
  (if (`self.DebuggingArcs?`)
    (`SceneComponent.SetVisibility` (`self.TestingArrow`) false false))
  (bind _output_get (set `self.DrawArcActivated?` false))
  (`self.RenderDecal` (and _output_get (`/Game/LOTAssets/TankAssets/Blueprints/LBX1Pawn_BP.TurretCamActive?` (`self.OwningPawn`))))
  (goto _label :!via `Break`))

(fn `GetArcSegmentAtTime`
  (params (MuzzleLocation :type "Vector Structure") (InitialVelocity :type "Vector Structure") (Gravity :type "Vector Structure") (Time1 :type "Float (double-precision)") (Time2 :type "Float (double-precision)"))
  (returns (Point1 :type "Vector Structure") (Point2 :type "Vector Structure"))
  ;[1 1 1] Get Arc Segment at Time
  (return (+ MuzzleLocation (* InitialVelocity Time1) (* Gravity (* Time1 Time1 0.5))) (+ MuzzleLocation (* InitialVelocity Time2) (* Gravity (* Time2 Time2 0.5)))))

(fn `RenderArcSegment`
  (params (Point1in :type "Vector Structure") (Point2in :type "Vector Structure") (DrawTypein :type "/Game/LOTAssets/TankAssets/Blueprints/Components/LBXArcDrawType_ENUM Enum") (LoopIndex :type Integer))
  (locals (Point1 :type "Vector Structure") (Point2 :type "Vector Structure") (DrawType :type "/Game/LOTAssets/TankAssets/Blueprints/Components/LBXArcDrawType_ENUM Enum"))
  ;[1 1 1] Render Segment
  (set `local.Point1` Point1in)
  (set `local.Point2` Point2in)
  (if (== (mod LoopIndex (`self.LineSegmentCount`)) 0)
    (switch `/Game/LOTAssets/TankAssets/Blueprints/Components/LBXArcDrawType_ENUM` DrawTypein
      (:`NewEnumerator0`
        (`KismetSystemLibrary.DrawDebugLine` (`local.Point1`) (`local.Point2`) (`self.ArcLineColor`) 0.0 (`self.ArcLineThickness`))))))

(fn `RenderDecal`
  (params (`IsVisible?` :type Boolean))
  ;[1 1 1] Render Decal
  (`SceneComponent.SetVisibility` (`self.ArcDecal`) `IsVisible?` false))