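; Player-controlled six-wheeled tank pawn with switchable cannon and mortar, battle and turret cameras with zoom, and health.
; BeginPlay wires meshes into movement, suspension, weapon and arc-aiming components, which handle driving, turret aim and firing, with the aim arc drawn for the mortar.
; The construction script applies configurable dynamic materials and arc color.
; Tick triggers death once, disabling input, removing components, and detaching turret and some wheels as physics debris with explosion effects.
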(event `self.ReceiveBeginPlay`
  ;[1 0.1339 0.9812] Begin Play
  ;;[1 1 1] Non Essential - Used for Experiments with projectile tagging
  (set `self.RandomProjectileTag` (+ (`KismetMathLibrary.RandomFloatInRange` 0.1 1500.0) (`KismetMathLibrary.RandomFloatInRange` 0.1 1500.0)))
  (if (`self.Debugging?`)
    (set `/Game/LOTAssets/TankAssets/Blueprints/Components/LBXArcAiming.DebuggingArcs?` true (`self.LBXArcAiming`))
    (set `/Game/LOTAssets/TankAssets/Blueprints/Components/LBXSuspension.DebugTraceLines` "ForOneFrame" (`self.LBXSuspension`))
    (`KismetSystemLibrary.PrintString` (`KismetStringLibrary.Concat_StrStr` "Approximate Vehicle Weight: " (`KismetStringLibrary.Conv_DoubleToString` (`PrimitiveComponent.GetMass` (`self.Body`)))) true true (struct :`R` 1.0 :`G` 0.773006 :`A` 1.0) 10.0)
    (`KismetSystemLibrary.PrintString` (`KismetStringLibrary.Concat_StrStr` "Random Projectile Tag: " (`KismetStringLibrary.Conv_DoubleToString` (`self.RandomProjectileTag`))) true true (struct :`G` 0.66 :`B` 1.0 :`A` 1.0) 10.0))
  (bind _output_get (set `self.LeftWheels` (`|MakeArray` (`self.Wheel4`) (`self.Wheel5`) (`self.Wheel6`))))
  (set `/Game/LOTAssets/TankAssets/Blueprints/Components/LBXMovement.LeftWheels` _output_get (`self.LBXMovement`))
  (bind _output_get_2 (set `self.RightWheels` (`|MakeArray` (`self.Wheel1`) (`self.Wheel2`) (`self.Wheel3`))))
  (set `/Game/LOTAssets/TankAssets/Blueprints/Components/LBXMovement.RightWheels` _output_get_2 (`self.LBXMovement`))
  (bind _output_get_3 (set `self.AllWheels` (`|MakeArray` (`self.Wheel1`) (`self.Wheel2`) (`self.Wheel3`) (`self.Wheel4`) (`self.Wheel5`) (`self.Wheel6`))))
  (set `/Game/LOTAssets/TankAssets/Blueprints/Components/LBXMovement.AllWheels` _output_get_3 (`self.LBXMovement`))
  (set `/Game/LOTAssets/TankAssets/Blueprints/Components/LBXMovement.TurretMesh` (`self.Turret`) (`self.LBXMovement`))
  (bind _output_get_4 (set `/Game/LOTAssets/TankAssets/Blueprints/Components/LBXMovement.BarrelMesh` (`self.Barrel`) (`self.LBXMovement`)))
  (set `/Game/LOTAssets/TankAssets/Blueprints/Components/LBXWeapons.BarrelMesh` _output_get_4 (`self.LBXWeapons`))
  (set `/Game/LOTAssets/TankAssets/Blueprints/Components/LBXArcAiming.ArcDecal` (`self.ArcAimDecal`) (`self.LBXArcAiming`))
  (set `/Game/LOTAssets/TankAssets/Blueprints/Components/LBXArcAiming.ArcBeam` (`self.ArcAimBeam`) (`self.LBXArcAiming`))
  (set `/Game/LOTAssets/TankAssets/Blueprints/Components/LBXArcAiming.TestingArrow` (`self.TestingArrow`) (`self.LBXArcAiming`))
  (set `/Game/LOTAssets/TankAssets/Blueprints/Components/LBXSuspension.EnableSuspension?` (`self.EnableSuspension?`) (`self.LBXSuspension`))
  (if (`self.EnableFlipCorrection?`)
    (`PrimitiveComponent.SetCenterOfMass` (`self.Body`) (0.0 0.0 -150.0) "None")))

(event `InputAction|SwitchCamera`
  (params (Key :type "Key Structure" :default "AnyKey"))
  ;[1 1 0] Camera Switching - Toggle Turret Cam
  (:`Pressed`
    (`self.EnableTurretCam` (not (`self.TurretCamActive?`)))))

(event `InputAction|PauseGame` :paused true
  (params (Key :type "Key Structure" :default "AnyKey"))
  ;[0 1 0.1843] Pausing and Unpausing Game
  (:`Pressed`
    (`/Engine/EditorBlueprintResources/StandardMacros.FlipFlop`
      (:`A`
        (`KismetSystemLibrary.PrintString` "Game Paused")
        (`GameplayStatics.SetGamePaused` true))
      (:`B`
        (`KismetSystemLibrary.PrintString` "Game Unpaused")
        (`GameplayStatics.SetGamePaused` false)))))

(event `self.ReceiveAnyDamage`
  (params (Damage :type "Float (single-precision)") (DamageType :type "DamageType Object Reference") (InstigatedBy :type "Controller Object Reference") (DamageCauser :type "Actor Object Reference"))
  ;[0.03979 1 0.9809] Event Any Damage
  (if (not (`self.IsDead?`))
    (set `self.CurrentHealth` (- (`self.CurrentHealth`) Damage))
    (if (`self.Debugging?`)
      (`KismetSystemLibrary.PrintString` (`KismetStringLibrary.Concat_StrStr` "Damage Received: " (`KismetStringLibrary.Conv_DoubleToString` Damage)) true true (struct :`R` 0.68 :`G` 0.1462 :`B` 0.1462 :`A` 1.0) 5.0)
      (`KismetSystemLibrary.PrintString` (`KismetStringLibrary.Concat_StrStr` "Current Health after damage: " (`KismetStringLibrary.Conv_DoubleToString` (`self.CurrentHealth`))) true true (struct :`G` 1.0 :`A` 1.0) 5.0))))

(event `InputAxis|LookRight`
  (params (AxisValue :type "Float (single-precision)"))
  ;[0 0 1] Turret Movement
  (`/Game/LOTAssets/TankAssets/Blueprints/Components/LBXMovement.TurretMovementHandler` (`self.LBXMovement`) AxisValue))

(event `InputAxis|LookUp`
  (params (AxisValue :type "Float (single-precision)"))
  ;[0 0 1] Barrel Movement
  (`/Game/LOTAssets/TankAssets/Blueprints/Components/LBXMovement.BarrelMovementHandler` (`self.LBXMovement`) AxisValue))

(event `Key|O`
  (params (Key :type "Key Structure" :default "AnyKey"))
  ;[1 1 1] "O" Key - Not zero...used for testing --- self-destruct
  (:`Pressed`
    (if (`self.Debugging?`)
      (set `self.CurrentHealth` 0.0))))

(event `InputAxis|MoveForward`
  (params (AxisValue :type "Float (single-precision)"))
  ;[0 1 0] Forward Movement
  (`/Game/LOTAssets/TankAssets/Blueprints/Components/LBXMovement.ForwardMovementHandler` (`self.LBXMovement`) AxisValue))

(event `InputAxis|MoveRight`
  (params (AxisValue :type "Float (single-precision)"))
  ;[0 1 0] Vehicle Turning Movement
  (`/Game/LOTAssets/TankAssets/Blueprints/Components/LBXMovement.TurningMovementHandler` (`self.LBXMovement`) AxisValue))

(event `self.ReceiveTick`
  (params (DeltaSeconds :type "Float (single-precision)"))
  ;[1 1 1] Event Tick
  (if (<= (`self.CurrentHealth`) 0.0)
    (`/Engine/EditorBlueprintResources/StandardMacros.DoOnce` false
      (:`Completed`
        (if (`self.Debugging?`)
          (`KismetSystemLibrary.PrintString` (`KismetStringLibrary.Concat_StrStr` (`KismetSystemLibrary.GetDisplayName` (`self.GetController`)) "is DEAD!") true true (struct :`R` 1.0 :`A` 1.0) 5.0))
        (`ActorComponent.Activate` (`self.BattleCam`) false)
        (`ActorComponent.Deactivate` (`self.TurretCam`))
        (`self.DeathSequence`)
        (set `self.IsDead?` true)))))

(event `InputAction|FireWeapon`
  (params (Key :type "Key Structure" :default "AnyKey"))
  ;[1 0 0] Weapon Switching, Fire Weapon, Zoom Camera
  (:`Pressed`
    (if (`self.CannonActive?`)
      (`/Game/LOTAssets/TankAssets/Blueprints/Components/LBXWeapons.FireMainCannon` (`self.LBXWeapons`))
      (else
        (`/Game/LOTAssets/TankAssets/Blueprints/Components/LBXWeapons.FireMortar` (`self.LBXWeapons`))))))

(event `InputAction|CameraZoom`
  (params (Key :type "Key Structure" :default "AnyKey"))
  (bind _battlecam (`self.BattleCam`))
  (bind _turretcam (`self.TurretCam`))
  ;[1 0 0] Weapon Switching, Fire Weapon, Zoom Camera
  (:`Pressed`
    (`/Engine/EditorBlueprintResources/StandardMacros.FlipFlop`
      (:`A`
        (set `CameraComponent.FieldOfView` (`self.CameraZoom`) _turretcam)
        (set `CameraComponent.FieldOfView` (`self.CameraZoom`) _battlecam))
      (:`B`
        (set `CameraComponent.FieldOfView` 90.0 _turretcam)
        (set `CameraComponent.FieldOfView` 90.0 _battlecam)))))

(event `InputAction|SwitchWeapons`
  (params (Key :type "Key Structure" :default "AnyKey"))
  (bind _lbxarcaiming (`self.LBXArcAiming`))
  (bind _returnvalue (`PlayerController.GetHUD` (`GameplayStatics.GetPlayerController` 0)))
  ;[1 0 0] Weapon Switching, Fire Weapon, Zoom Camera
  (:`Pressed`
    (`/Engine/EditorBlueprintResources/StandardMacros.FlipFlop`
      (:`A`
        (set `self.CannonActive?` false)
        (bind _aslbxhud_bp (cast `/Game/LOTAssets/TankAssets/Blueprints/LBXHUD_BP` _returnvalue))
        (bind _returnvalue_2 (`Image.GetDynamicMaterial` (`/Game/LOTAssets/TankAssets/Blueprints/LBXHUDWidget_BP.ProjectileImage` (`/Game/LOTAssets/TankAssets/Blueprints/LBXHUD_BP.HUDWidget` _aslbxhud_bp))))
        (`MaterialInstanceDynamic.SetTextureParameterValue` _returnvalue_2 "WeaponIcon" "/Game/LOTAssets/TankAssets/Textures/T_MortarIcon.T_MortarIcon")
        (`/Game/LOTAssets/TankAssets/Blueprints/Components/LBXArcAiming.DrawArcPath` _lbxarcaiming)
        (set `/Game/LOTAssets/TankAssets/Blueprints/Components/LBXWeapons.CurrentProjectile` "/Game/LOTAssets/TankAssets/Blueprints/LBXMortarStage1_BP.LBXMortarStage1_BP_C" (`self.LBXWeapons`)))
      (:`B`
        (set `self.CannonActive?` true)
        (bind _aslbxhud_bp_2 (cast `/Game/LOTAssets/TankAssets/Blueprints/LBXHUD_BP` _returnvalue))
        (bind _returnvalue_3 (`Image.GetDynamicMaterial` (`/Game/LOTAssets/TankAssets/Blueprints/LBXHUDWidget_BP.ProjectileImage` (`/Game/LOTAssets/TankAssets/Blueprints/LBXHUD_BP.HUDWidget` _aslbxhud_bp_2))))
        (`MaterialInstanceDynamic.SetTextureParameterValue` _returnvalue_3 "WeaponIcon" "/Game/LOTAssets/TankAssets/Textures/T_HighVelocityIcon.T_HighVelocityIcon")
        (`/Game/LOTAssets/TankAssets/Blueprints/Components/LBXArcAiming.BreakArcPathDraw` _lbxarcaiming)))))

(fn `DeathSequence`
  (bind _wheel1 (`self.Wheel1`))
  ;[1 0.1339 0.9812] Death Sequence
  ;[1 1 1] Disable Player Input on Death
  (`self.DisableInput` null)
  ;[1 1 1] Allows for camera to be used after death without following turret
  (`SceneComponent.DetachFromParent` (`self.BattleCam`) true true)
  ;[1 1 1] Deactivates all components and destroys barrel
  (`ActorComponent.Deactivate` (`self.LBXSuspension`))
  (`ActorComponent.Deactivate` (`self.LBXMovement`))
  (`ActorComponent.Deactivate` (`self.LBXWeapons`))
  (`ActorComponent.Deactivate` (`self.LBXArcAiming`))
  (`ActorComponent.K2_DestroyComponent` (`self.Barrel`))
  (`ActorComponent.K2_DestroyComponent` (`self.LBXMovement`))
  (`ActorComponent.K2_DestroyComponent` (`self.LBXWeapons`))
  (`ActorComponent.K2_DestroyComponent` (`self.LBXArcAiming`))
  (`ActorComponent.K2_DestroyComponent` (`self.LBXSuspension`))
  ;[1 1 1] Add relative location to wheels 1, 4 and 6 so physics can be enabled after death
  (`SceneComponent.K2_AddRelativeLocation` (`self.Wheel4`) (-100.0 0.0 0.0) false false)
  (`SceneComponent.K2_AddRelativeLocation` (`self.Wheel1`) (100.0 0.0 0.0) false false)
  (`SceneComponent.K2_AddRelativeLocation` (`self.Wheel6`) (100.0 0.0 0.0) false false)
  ;[1 1 1] Detach Turret, and wheels 1, 4 and 6 from parrent and set simulate physics to true
  (`SceneComponent.DetachFromParent` _wheel1 false true)
  (`SceneComponent.DetachFromParent` (`self.Wheel6`) false true)
  (`SceneComponent.DetachFromParent` (`self.Wheel4`) false true)
  (`SceneComponent.DetachFromParent` (`self.Turret`) false true)
  (`PrimitiveComponent.SetSimulatePhysics` _wheel1 true)
  (`PrimitiveComponent.SetSimulatePhysics` (`self.Wheel6`) true)
  (`PrimitiveComponent.SetSimulatePhysics` (`self.Wheel4`) true)
  (`PrimitiveComponent.SetSimulatePhysics` (`self.Turret`) true)
  ;[1 1 1] Sound and Particle Emitters spawned  at death
  (`GameplayStatics.SpawnSoundAttached` (`self.DeathExplosionSound`) (`self.Body`))
  (`GameplayStatics.SpawnEmitterAttached` (`self.DeathExplosionEmitter`) (`self.Body`) "Turret" (0.0 0.0 0.0) (struct) "SnapToTarget")
  (`GameplayStatics.SpawnEmitterAttached` (`self.DeathSmokeEmitter`) (`self.Body`) "None" (0.0 0.0 0.0) (struct) "SnapToTarget")
  (`GameplayStatics.SpawnEmitterAttached` (`self.DeathSmokeEmitter`) (`self.Body`) "Turret" (0.0 0.0 0.0) (struct) "SnapToTarget")
  ;[1 1 1] Timer delay on destroy actor
  (`KismetSystemLibrary.K2_SetTimerDelegate` (`|CreateDelegate` :!event `K2_DestroyActor`) (`self.TimeAfterDeath`)))

(fn `EnableTurretCam`
  (params (`Current State` :type Boolean))
  (bind _battlecam (`self.BattleCam`))
  (bind _turretcam (`self.TurretCam`))
  (bind _returnvalue (`PlayerController.GetHUD` (`GameplayStatics.GetPlayerController` 0)))
  ;[1 0.1339 0.9812] Enable Turret Cam
  (set `self.TurretCamActive?` `Current State`)
  (if (`self.TurretCamActive?`)
    (bind _aslbxhud_bp (cast `/Game/LOTAssets/TankAssets/Blueprints/LBXHUD_BP` _returnvalue))
    (set `/Game/LOTAssets/TankAssets/Blueprints/LBXHUD_BP.TurretCamCrosshairs?` true _aslbxhud_bp)
    (`ActorComponent.Activate` _turretcam false)
    (set `CameraComponent.FieldOfView` 90.0 _turretcam)
    (`ActorComponent.Deactivate` (`self.BattleCam`))
    (else
      (bind _aslbxhud_bp_2 (cast `/Game/LOTAssets/TankAssets/Blueprints/LBXHUD_BP` _returnvalue))
      (set `/Game/LOTAssets/TankAssets/Blueprints/LBXHUD_BP.TurretCamCrosshairs?` false _aslbxhud_bp_2)
      (`ActorComponent.Deactivate` (`self.TurretCam`))
      (`ActorComponent.Activate` _battlecam false)
      (set `CameraComponent.FieldOfView` 90.0 _battlecam))))

(fn `UserConstructionScript`
  (bind _arcaimcolor (`self.ArcAimColor`))
  ;[1 0.1339 0.9812] Construction Script Start
  ;[0 1 0.1843] Dynamic Material assigment to vehicle parts
  (bind _returnvalue (`PrimitiveComponent.CreateDynamicMaterialInstance` (`self.Body`) 1 (`self.MasterMaterial`)))
  (set `self.BodyMaterial` _returnvalue)
  (bind _returnvalue_2 (`PrimitiveComponent.CreateDynamicMaterialInstance` (`self.Turret`) 0 (`self.MasterMaterial`)))
  (set `self.TurretMaterial` _returnvalue_2)
  (bind _returnvalue_3 (`PrimitiveComponent.CreateDynamicMaterialInstance` (`self.Barrel`) 0 (`self.MasterMaterial`)))
  (set `self.BarrelMaterial` _returnvalue_3)
  ;[0 1 0] Sets Color Texture and Material Metallic and Roughness settings
  (`MaterialInstanceDynamic.SetTextureParameterValue` (`self.BodyMaterial`) "ColorTexture" (`self.ColorTexture`))
  (`MaterialInstanceDynamic.SetTextureParameterValue` (`self.TurretMaterial`) "ColorTexture" (`self.ColorTexture`))
  (`MaterialInstanceDynamic.SetTextureParameterValue` (`self.BarrelMaterial`) "ColorTexture" (`self.ColorTexture`))
  (`MaterialInstanceDynamic.SetScalarParameterValue` (`self.BodyMaterial`) "Metallic" (`self.MaterialMetallicValue`))
  (`MaterialInstanceDynamic.SetScalarParameterValue` (`self.TurretMaterial`) "Metallic" (`self.MaterialMetallicValue`))
  (`MaterialInstanceDynamic.SetScalarParameterValue` (`self.BarrelMaterial`) "Metallic" (`self.MaterialMetallicValue`))
  (`MaterialInstanceDynamic.SetScalarParameterValue` (`self.BodyMaterial`) "Roughness" (`self.MaterialRoughnessValue`))
  (`MaterialInstanceDynamic.SetScalarParameterValue` (`self.TurretMaterial`) "Roughness" (`self.MaterialRoughnessValue`))
  (`MaterialInstanceDynamic.SetScalarParameterValue` (`self.BarrelMaterial`) "Roughness" (`self.MaterialRoughnessValue`))
  ;[1 1 1] Sets color of Aim endpoint decal and Arc line color
  (bind _returnvalue_4 (`DecalComponent.CreateDynamicMaterialInstance` (`self.ArcAimDecal`)))
  (`MaterialInstanceDynamic.SetVectorParameterValue` _returnvalue_4 "Color" _arcaimcolor)
  (set `/Game/LOTAssets/TankAssets/Blueprints/Components/LBXArcAiming.ArcLineColor` _arcaimcolor (`self.LBXArcAiming`)))