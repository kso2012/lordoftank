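; First-stage LBX mortar projectile that bursts into a cluster of LBXMortarStage2_BP submunitions.
; It launches at a set local velocity with an attached trail, pitches along its velocity each tick, and destroys itself on hitting actors lacking its tags.
; EndPlay applies radial damage, plays release effects and spawns submunitions at randomized angles.
; That spawn loop also restores HUD crosshairs and clears the pawn's follow-cam flag.
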(event `self.ReceiveBeginPlay`
  ;[1 0.1339 0.9812] Event Begin Play
  (`ProjectileMovementComponent.SetVelocityInLocalSpace` (`self.ProjectileMovement`) (`self.InitialVelocity`))
  (`GameplayStatics.SpawnEmitterAttached` (`self.MortarTravelEmitter`) (`self.MortarMesh`) "None" (0.0 0.0 0.0) (struct) "SnapToTargetIncludingScale"))

(event `self.ReceiveTick`
  (params (DeltaSeconds :type "Float (single-precision)"))
  ;[1 1 1] Event Tick
  (`self.ProjectilePitchUpdate`))

(event `self.ReceiveHit`
  (params (MyComp :type "PrimitiveComponent Object Reference") (Other :type "Actor Object Reference") (OtherComp :type "PrimitiveComponent Object Reference") (bSelfMoved :type Boolean) (HitLocation :type "Vector Structure") (HitNormal :type "Vector Structure") (NormalImpulse :type "Vector Structure") (Hit :type "HitResult Structure (by ref)"))
  ;[1 1 1] Event Hit
  (for _array_element (`self.Tags`)
    (if (not (`self.ActorHasTag` Other _array_element))
      (`self.K2_DestroyActor`))))

(event `self.ReceiveEndPlay`
  (params (EndPlayReason :type "EEndPlayReason Enum" :default "Destroyed"))
  (bind _returnvalue (`self.K2_GetActorLocation`))
  ;[1 1 1] Event End Play
  (`GameplayStatics.ApplyRadialDamage` :`BaseDamage` (`self.DamageDealt`) :`Origin` (`self.K2_GetActorLocation`) :`DamageRadius` (`self.DamageRadius`) :`bDoFullDamage` true)
  (`GameplayStatics.SpawnEmitterAtLocation` (`self.Stage2ReleaseEmitter`) _returnvalue)
  (`GameplayStatics.SpawnSoundAtLocation` (`self.Stage2ReleaseSound`) _returnvalue)
  (for _ (range (+ (`self.NumberOfStage2Units`) 1))
    (`|SpawnActorFromClass` "/Game/LOTAssets/TankAssets/Blueprints/LBXMortarStage2_BP.LBXMortarStage2_BP_C" (`KismetMathLibrary.MakeTransform` (+ _returnvalue (`KismetMathLibrary.RandomFloatInRange` 5.0 25.0)) (`KismetMathLibrary.MakeRotator` 0.0 (`KismetMathLibrary.RandomFloatInRange` 30.0 75.0) (`KismetMathLibrary.RandomFloatInRange` -180.0 180.0))) "Undefined" "OverrideRootScale")
    ;[1 0.773 0] This turns crosshairs back on if the follow cam was used
    (bind _aslbxhud_bp (cast `/Game/LOTAssets/TankAssets/Blueprints/LBXHUD_BP` (`PlayerController.GetHUD` (`GameplayStatics.GetPlayerController` 0))))
    (if (!= (`/Game/LOTAssets/TankAssets/Blueprints/LBXHUD_BP.ShowCrosshairs` _aslbxhud_bp) true)
      (set `/Game/LOTAssets/TankAssets/Blueprints/LBXHUD_BP.ShowCrosshairs` true _aslbxhud_bp)
      (bind _aslbx1pawn_bp (cast `/Game/LOTAssets/TankAssets/Blueprints/LBX1Pawn_BP` (`GameplayStatics.GetPlayerPawn` 0)))
      (bind _lbxweapons (`/Game/LOTAssets/TankAssets/Blueprints/LBX1Pawn_BP.LBXWeapons` _aslbx1pawn_bp))
      (if (!= (`/Game/LOTAssets/TankAssets/Blueprints/Components/LBXWeapons.FollowCamActive?` _lbxweapons) false)
        (set `/Game/LOTAssets/TankAssets/Blueprints/Components/LBXWeapons.FollowCamActive?` false _lbxweapons)))))

(event `ProjectilePitchUpdate`
  (bind (_returnvalue_roll _returnvalue_pitch _returnvalue_yaw) (`KismetMathLibrary.BreakRotator` (`self.K2_GetActorRotation`)))
  (bind (_returnvalue_roll_2 _returnvalue_pitch_2) (`KismetMathLibrary.BreakRotator` (`KismetMathLibrary.MakeRotFromX` (`self.GetVelocity`))))
  ;[0.03979 1 0.9809] Projectile Pitch Update
  (`self.K2_SetActorRotation` (`KismetMathLibrary.MakeRotator` _returnvalue_roll _returnvalue_pitch_2 _returnvalue_yaw)))

(fn `UserConstructionScript`)