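; LBXHUD_BP is a HUD Blueprint that shows the main HUD widget and draws a screen-centred crosshair.
; On Begin Play it creates LBXHUDWidget_BP, stores it and adds it to the viewport.
; Each Draw HUD pass, when crosshairs are enabled, picks the turret-cam or battle-cam texture from a flag and draws it centred using the screen size and texture size.
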(event `self.ReceiveBeginPlay`
  ;[1 0.1339 0.9812] Event Begin Play
  (bind _returnvalue (`|CreateWidget` "/Game/LOTAssets/TankAssets/Blueprints/LBXHUDWidget_BP.LBXHUDWidget_BP_C"))
  (set `self.HUDWidget` _returnvalue)
  (`UserWidget.AddToViewport` (`self.HUDWidget`) 0))

(event `self.ReceiveDrawHUD`
  (params (SizeX :type Integer) (SizeY :type Integer))
  (bind _texturesize (`self.TextureSize`))
  (bind _returnvalue (`KismetMathLibrary.FTrunc` (/ (`self.TextureSize`) 2.0)))
  ;[1 0.1339 0.9812] Event Receive Draw HUD
  (set `self.SizeX` SizeX)
  (set `self.SizeY` SizeY)
  (if (`self.ShowCrosshairs`)
    (if (`self.TurretCamCrosshairs?`)
      (set `self.CurrentCrosshairTexture` (`self.TurretCamCrosshair`))
      (else
        (set `self.CurrentCrosshairTexture` (`self.BattleCamCrosshair`))))
    (`self.DrawTexture` (`self.CurrentCrosshairTexture`) (`KismetMathLibrary.Conv_IntToDouble` (- (/ (`self.SizeX`) 2) _returnvalue)) (`KismetMathLibrary.Conv_IntToDouble` (- (/ (`self.SizeY`) 2) _returnvalue)) _texturesize _texturesize 0.0 0.0 1.0 1.0 (struct :`R` 1.0 :`G` 1.0 :`B` 1.0 :`A` 1.0) "BLEND_Translucent" 1.0 true)))

(fn `UserConstructionScript`)