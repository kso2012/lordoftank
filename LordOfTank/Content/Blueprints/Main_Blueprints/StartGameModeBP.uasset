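; Game mode for the start menu, handling server connection and entry into the multiplayer level.
; Spawns and destroys actor-based main menu, keypad, lobby and room screens at stored transforms.
; ClickEnt reuses one keypad text box, first for the IP address, then for the nickname before opening the room, delegating both to LOTGameInstance.
; Tick polls the instance's IsStart flag, then shows a loading screen and opens MultiTest after a delay.
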(event `self.ReceiveBeginPlay`
  (`self.SpawnMainMenu`))

(event `ClickEnt`
  (bind _aslotgame_instance (cast `LOTGameInstance` (`GameplayStatics.GetGameInstance`)))
  (bind _askeypad_display (cast `/Game/Blueprints/Main_Blueprints/KeypadDisplay` (`self.KeypadDiplayPT`)))
  (bind _askeypad_display_wb (cast `/Game/Blueprints/Main_Blueprints/KeypadDisplayWB` (`WidgetComponent.GetUserWidgetObject` (`/Game/Blueprints/Main_Blueprints/KeypadDisplay.Widget` _askeypad_display))))
  (if (`LOTGameInstance.bIsConnected` _aslotgame_instance)
    (bind _editabletextbox_0 (`/Game/Blueprints/Main_Blueprints/KeypadDisplayWB.EditableTextBox_0` _askeypad_display_wb))
    (bind _returnvalue (`KismetTextLibrary.Conv_TextToString` (`EditableTextBox.GetText` _editabletextbox_0)))
    (set `LOTGameInstance.Nickname` _returnvalue _aslotgame_instance)
    (`LOTGameInstance.ClickNameEntBT` _aslotgame_instance)
    (bind _asstart_game_mode_bp (cast `/Game/Blueprints/Main_Blueprints/StartGameModeBP` (`GameplayStatics.GetGameMode`)))
    (`GameplayStatics.SpawnSound2D` "/Game/ProjectilesPack/Sounds/Environment/Target_Destroyed_Cue.Target_Destroyed_Cue")
    (`self.DestroyKeyPad` _asstart_game_mode_bp)
    (`self.SpawnRoom` _asstart_game_mode_bp)
    (else
      (set `LOTGameInstance.IPaddr` _returnvalue _aslotgame_instance)
      (bind _returnvalue_2 (`LOTGameInstance.ClickIpEntBT` _aslotgame_instance))
      (if _returnvalue_2
        (set `LOTGameInstance.bIsConnected` true _aslotgame_instance)
        (`GameplayStatics.SpawnSound2D` "/Game/ProjectilesPack/Sounds/Environment/Target_Destroyed_Cue.Target_Destroyed_Cue")
        (else
          (`KismetSystemLibrary.Delay` 0.5)
          (`GameplayStatics.SpawnSound2D` "/Game/ProjectilesPack/Sounds/Common/BladeImpact.BladeImpact")))
      (`EditableTextBox.SetText` _editabletextbox_0 ""))))

(event `self.ReceiveTick`
  (params (DeltaSeconds :type "Float (single-precision)"))
  (if (not (`self.isLoad`))
    (bind _aslotgame_instance (cast `LOTGameInstance` (`GameplayStatics.GetGameInstance`)))
    (if (`LOTGameInstance.bIsStart` _aslotgame_instance)
      (set `self.isLoad` true)
      (`GameplayStatics.SpawnSound2D` "/Game/ProjectilesPack/Sounds/Common/BladeSwarmInit.BladeSwarmInit")
      (`|SpawnActorFromClass` "/Game/Blueprints/Main_Blueprints/LoadingScreen.LoadingScreen_C" (`self.NewVar_0`) "Undefined" "OverrideRootScale")
      (`KismetSystemLibrary.Delay` 3.0)
      (`GameplayStatics.OpenLevel` "MultiTest"))))

(fn `DestroyKeyPad`
  (`self.K2_DestroyActor` (`self.KeypadPT`))
  (`self.K2_DestroyActor` (`self.KeypadDiplayPT`)))

(fn `DestroyLobby`
  (`self.K2_DestroyActor` (`self.LobbyPT`)))

(fn `DestroyMainMenu`
  (`self.K2_DestroyActor` (`self.MainMenuPT`)))

(fn `DestroyRoom`
  (`self.K2_DestroyActor` (`self.RoomPT`)))

(fn `SpawnKeyPad`
  (bind _returnvalue (`|SpawnActorFromClass` "/Game/Blueprints/Main_Blueprints/Keypad.Keypad_C" (`self.KeypadLC`) "Undefined" "OverrideRootScale"))
  (set `self.KeypadPT` _returnvalue)
  (bind _returnvalue_2 (`|SpawnActorFromClass` "/Game/Blueprints/Main_Blueprints/KeypadDisplay.KeypadDisplay_C" (`self.KeypadDisplayLC`) "Undefined" "OverrideRootScale"))
  (set `self.KeypadDiplayPT` _returnvalue_2))

(fn `SpawnLobby`
  (bind _returnvalue (`|SpawnActorFromClass` "/Game/Blueprints/Main_Blueprints/LobbyDisplay.LobbyDisplay_C" (`self.LobbyMenuLC`) "Undefined" "OverrideRootScale"))
  (set `self.LobbyPT` _returnvalue))

(fn `SpawnMainMenu`
  (bind _returnvalue (`|SpawnActorFromClass` "/Game/Blueprints/Main_Blueprints/Menu_Actor.Menu_Actor_C" (`self.MainMenuLC`) "Undefined" "OverrideRootScale"))
  (set `self.MainMenuPT` _returnvalue))

(fn `SpawnRoom`
  (bind _returnvalue (`|SpawnActorFromClass` "/Game/Blueprints/Main_Blueprints/RoomDisplay.RoomDisplay_C" (`self.RoomLC`) "Undefined" "OverrideRootScale"))
  (set `self.RoomPT` _returnvalue))

(fn `UserConstructionScript`)