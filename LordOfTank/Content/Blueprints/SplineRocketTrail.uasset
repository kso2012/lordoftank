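; SplineRocketTrail is a construction-script Blueprint that stretches a configurable static mesh along a single spline mesh segment between Start and End, apparently as a rocket trail.
; Tangents point from Start toward StartTangent and from EndTangent toward End, scaled by the Start-to-End distance.
; AutoTangents normalizes those directions first; otherwise handle length also affects curvature.
; It also applies roll at both ends and an optional material override.
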(fn `UserConstructionScript`
  (bind _autotangents (`self.AutoTangents`))
  (bind _splinemesh1 (`self.SplineMesh1`))
  (bind _material (`self.Material`))
  (bind _splinemesh1_2 (`self.SplineMesh1`))
  (bind _location (.location (`self.Start`)))
  (bind _location_2 (.location (`self.End`)))
  (bind _returnvalue (- _location_2 (`self.EndTangent`)))
  (bind _returnvalue_2 (- (`self.StartTangent`) _location))
  (bind _returnvalue_3 (`KismetMathLibrary.VSize` (- _location_2 _location)))
  (`StaticMeshComponent.SetStaticMesh` _splinemesh1 (`self.StaticMesh`))
  (`SplineMeshComponent.SetStartAndEnd` _splinemesh1 _location (`KismetMathLibrary.SelectVector` (* (`KismetMathLibrary.Normal` _returnvalue_2) _returnvalue_3) (* _returnvalue_2 (/ _returnvalue_3 200.0)) _autotangents) _location_2 (`KismetMathLibrary.SelectVector` (* (`KismetMathLibrary.Normal` _returnvalue) _returnvalue_3) (* _returnvalue (/ _returnvalue_3 200.0)) _autotangents) true)
  (`SplineMeshComponent.SetStartRoll` _splinemesh1_2 (`self.StartRoll`) true)
  (`SplineMeshComponent.SetEndRoll` _splinemesh1_2 (`self.EndRoll`) true)
  (`/Engine/EditorBlueprintResources/StandardMacros.IsValid` _material
    (:`Is Valid`
      (`PrimitiveComponent.SetMaterial` (`self.SplineMesh1`) 0 _material))))