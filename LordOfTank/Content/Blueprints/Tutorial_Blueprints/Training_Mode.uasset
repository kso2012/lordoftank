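; Training_Mode is a tutorial Blueprint that tracks training state and switches player control between a tank and a drone.
; BeginPlay resets a collision counter and a shot-training progress flag, and GetCollision increments the counter.
; SetTank and SetDrone store the two pawn references.
; ChangePawn unpossesses the first player controller, then possesses the drone if given the tank, otherwise the tank.
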(event `self.ReceiveBeginPlay`
  (set `self.Collision Count` 0)
  (set `self.Shot Training Proceed` false))

(fn `Change Pawn`
  (params (Pawn :type "Pawn Object Reference"))
  (bind _returnvalue (`GameplayStatics.GetPlayerController` 0))
  (`Controller.UnPossess` _returnvalue)
  (if (== Pawn (`self.Tank_Pawn`))
    (`Controller.Possess` _returnvalue (`self.Drone_Pawn`))
    (else
      (`Controller.Possess` _returnvalue (`self.Tank_Pawn`)))))

(fn `Get Collision`
  (set `self.Collision Count` (+ (`self.Collision Count`) 1)))

(fn `Set Drone`
  (params (Drone :type "Pawn Object Reference"))
  (set `self.Drone_Pawn` Drone))

(fn `Set Tank`
  (params (Tank :type "Pawn Object Reference"))
  (set `self.Tank_Pawn` Tank))

(fn `UserConstructionScript`)