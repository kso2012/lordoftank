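; Training tank for the tutorial, stepping the player through a sequence of message panels tracked by TutorialLevel.
; E advances the panels, while Tick hides steps 4 and 10 after a delay and moves past step 10 once T sets Proceed.
; At step 11, E spawns and possesses a new Trainig_Tank, then moves the Training_Mode game mode to this tank's transform.
; Left mouse toggles ShotUIActor visibility.
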(event `self.ReceiveBeginPlay`
  (`|ExecutionSequence`
    (:`then_0`
      (set `self.Tutorial Level` 1)
      (set `self.Proceed` false)
      (`SceneComponent.SetVisibility` (`self.Tutorial1`) true false)
      (`SceneComponent.SetVisibility` (`self.E Message`) true false)
      (`self.EnableInput` (`GameplayStatics.GetPlayerController` 0)))))

(event `self.ReceiveTick`
  (params (DeltaSeconds :type "Float (single-precision)"))
  (if (== (`self.Tutorial Level`) 4)
    (`KismetSystemLibrary.Delay` 2.0)
    (if (== (`self.Tutorial Level`) 4)
      (`SceneComponent.SetVisibility` (`self.E Message`) false false)
      (`SceneComponent.SetVisibility` (`self.Tutorial4`) false false))
    (elif (== (`self.Tutorial Level`) 10)
      (if (`self.Proceed`)
        (set `self.Proceed` false)
        (set `self.Tutorial Level` 11)
        (`SceneComponent.SetVisibility` (`self.Tutorial11`) true false)
        (`SceneComponent.SetVisibility` (`self.E Message`) true false)
        (`SceneComponent.SetVisibility` (`self.Tutorial10`) false false)
        (set `self.Proceed10` true)
        (else
          (`KismetSystemLibrary.Delay` 2.0)
          (if (== (`self.Tutorial Level`) 10)
            (`SceneComponent.SetVisibility` (`self.Tutorial10`) false false)))))))

(event `Key|T`
  (params (Key :type "Key Structure" :default "AnyKey"))
  (:`Pressed`
    (set `self.Proceed` true)))

(event `Key|E`
  (params (Key :type "Key Structure" :default "AnyKey"))
  (:`Pressed`
    (if (== (`self.Tutorial Level`) 1)
      (set `self.Tutorial Level` 2)
      (`SceneComponent.SetVisibility` (`self.Tutorial1`) false false)
      (`SceneComponent.SetVisibility` (`self.Tutorial2`) true false)
      (elif (== (`self.Tutorial Level`) 2)
        (set `self.Tutorial Level` 3)
        (`SceneComponent.SetVisibility` (`self.Tutorial2`) false false)
        (`SceneComponent.SetVisibility` (`self.Tutorial3`) true false)
        (elif (== (`self.Tutorial Level`) 3)
          (set `self.Tutorial Level` 4)
          (`SceneComponent.SetVisibility` (`self.Tutorial3`) false false)
          (`SceneComponent.SetVisibility` (`self.Tutorial4`) true false)
          (elif (== (`self.Tutorial Level`) 4)
            (set `self.Tutorial Level` 5)
            (`SceneComponent.SetVisibility` (`self.Tutorial4`) false false)
            (`SceneComponent.SetVisibility` (`self.Tutorial5`) true false)
            (`SceneComponent.SetVisibility` (`self.E Message`) true false)
            (elif (== (`self.Tutorial Level`) 5)
              (set `self.Tutorial Level` 6)
              (`SceneComponent.SetVisibility` (`self.Tutorial5`) false false)
              (`SceneComponent.SetVisibility` (`self.Tutorial6`) true false)
              (elif (== (`self.Tutorial Level`) 6)
                (set `self.Tutorial Level` 7)
                (`SceneComponent.SetVisibility` (`self.Tutorial6`) false false)
                (`SceneComponent.SetVisibility` (`self.Tutorial7`) true false)
                (elif (== (`self.Tutorial Level`) 7)
                  (set `self.Tutorial Level` 8)
                  (`SceneComponent.SetVisibility` (`self.Tutorial7`) false false)
                  (`SceneComponent.SetVisibility` (`self.Tutorial8`) true false)
                  (elif (== (`self.Tutorial Level`) 8)
                    (set `self.Tutorial Level` 9)
                    (`SceneComponent.SetVisibility` (`self.Tutorial8`) false false)
                    (`SceneComponent.SetVisibility` (`self.Tutorial9`) true false)
                    (elif (== (`self.Tutorial Level`) 9)
                      (set `self.Tutorial Level` 10)
                      (`SceneComponent.SetVisibility` (`self.Tutorial9`) false false)
                      (`SceneComponent.SetVisibility` (`self.Tutorial10`) true false)
                      (`SceneComponent.SetVisibility` (`self.E Message`) false false)
                      (elif (`self.Proceed10`)
                        (if (== (`self.Tutorial Level`) 10)
                          (set `self.Tutorial Level` 11)
                          (`SceneComponent.SetVisibility` (`self.Tutorial11`) false false)
                          (`SceneComponent.SetVisibility` (`self.Tutorial12`) true false)
                          (elif (== (`self.Tutorial Level`) 11)
                            (bind _returnvalue (`|SpawnActorFromClass` "Trainig_Tank_C" (`self.Shot_Position`) "Undefined" "OverrideRootScale"))
                            (`Controller.Possess` (`GameplayStatics.GetPlayerController` 0) _returnvalue)
                            (bind _astraining_mode (cast `/Game/Blueprints/Tutorial_Blueprints/Training_Mode` (`GameplayStatics.GetGameMode`)))
                            (bind _output_get (set `self.Training_TankMode` _astraining_mode))
                            (`self.K2_SetActorTransform` _output_get (`self.GetTransform`) false false)
                            (set `self.Tutorial Level` 13)
                            (set `self.Proceed` false)
                            (`SceneComponent.SetVisibility` (`self.Tutorial1`) true false)
                            (`SceneComponent.SetVisibility` (`self.E Message`) true false)))))))))))))))

(event `Key|LeftMouseButton`
  (params (Key :type "Key Structure" :default "AnyKey"))
  (:`Pressed`
    (`SceneComponent.ToggleVisibility` (`self.Shot_UI_Actor`) true)))

(fn `UserConstructionScript`)