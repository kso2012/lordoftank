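; Tutorial shooting target with a pulsing center flash driven by a looping or one-shot timeline on text renders.
; Any damage, or a collision box hit while Training_Mode allows shot training, hides the X and flash markers and disables collision.
; Hits also notify Training_Mode.
; After a delay, markers and query-only collision return and a new destructible mesh component is added to respawn the target.
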(event `self.ReceiveBeginPlay`
  ;[1 1 1] Begin Play - Sets up a flash effect for the center of target
  (bind (_direction _flashalpha) (`Timeline|TargetFlash`)
    (:`Update`
      (`TextRenderComponent.SetTextRenderColor` (`self.TargetFlashBack`) (`KismetMathLibrary.Conv_LinearColorToColor` _flashalpha))
      (`TextRenderComponent.SetTextRenderColor` (`self.TargetFlashFront`) (`KismetMathLibrary.Conv_LinearColorToColor` _flashalpha)))))

(event `self.ReceiveAnyDamage`
  (params (Damage :type "Float (single-precision)") (DamageType :type "DamageType Object Reference") (InstigatedBy :type "Controller Object Reference") (DamageCauser :type "Actor Object Reference"))
  ;[1 1 1] Box Collision Overlap and Event Any Damage - Respawns Target Destructible Mesh after impacts
  (`SceneComponent.SetVisibility` (`self.TargetXFront`) false false :!label _label)
  (`SceneComponent.SetVisibility` (`self.TagetXBack`) false false)
  (`SceneComponent.SetVisibility` (`self.TargetFlashFront`) false false)
  (`SceneComponent.SetVisibility` (`self.TargetFlashBack`) false false)
  (set `self.isCollision` true)
  (`PrimitiveComponent.SetCollisionEnabled` (`self.CollisionBox`) "NoCollision")
  (`KismetSystemLibrary.Delay` 5.0)
  (`SceneComponent.SetVisibility` (`self.TagetXBack`) true false)
  (`SceneComponent.SetVisibility` (`self.TargetXFront`) true false)
  (`SceneComponent.SetVisibility` (`self.TargetFlashFront`) true false)
  (`SceneComponent.SetVisibility` (`self.TargetFlashBack`) true false)
  (bind _returnvalue (`AddComponent|NODE_AddDestructibleComponent-0` :`RelativeTransform` (`KismetMathLibrary.MakeTransform` (0.0 0.0 500.0))))
  (`PrimitiveComponent.SetCollisionEnabled` (`self.CollisionBox`) "QueryOnly")
  (`DestructibleComponent.SetDestructibleMesh` _returnvalue (`self.DestructibleMesh`))
  (set `self.isCollision` false))

(event `self.CollisionBox.OnComponentBeginOverlap`
  (params (OverlappedComponent :type "PrimitiveComponent Object Reference") (OtherActor :type "Actor Object Reference") (OtherComp :type "PrimitiveComponent Object Reference") (OtherBodyIndex :type Integer) (bFromSweep :type Boolean) (SweepResult :type "HitResult Structure (by ref)")))

(event `self.CollisionBox.OnComponentHit`
  (params (HitComponent :type "PrimitiveComponent Object Reference") (OtherActor :type "Actor Object Reference") (OtherComp :type "PrimitiveComponent Object Reference") (NormalImpulse :type "Vector Structure") (Hit :type "HitResult Structure (by ref)"))
  (if (not (`self.isCollision`))
    (bind _astraining_mode (cast `/Game/Blueprints/Tutorial_Blueprints/Training_Mode` (`GameplayStatics.GetGameMode`)))
    (if (`/Game/Blueprints/Tutorial_Blueprints/Training_Mode.Shot Training Proceed` _astraining_mode)
      (`/Game/Blueprints/Tutorial_Blueprints/Training_Mode.Get Collision` _astraining_mode)
      (goto _label))))

(fn `UserConstructionScript`)