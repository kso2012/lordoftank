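; Training tank actor that shows a two-step tutorial in the game.
; On begin play it sets the tutorial level to 1, shows the first tutorial and the E message component, and enables input from the first player controller.
; Pressing E at level 1 advances to level 2, swapping the first tutorial for the second while the E message stays visible.
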(event `self.ReceiveBeginPlay`
  (set `self.Tutorial Level` 1)
  (set `self.Proceed` false)
  (`SceneComponent.SetVisibility` (`self.Tutorial1`) true false)
  (`SceneComponent.SetVisibility` (`self.E Message`) true false)
  (`self.EnableInput` (`GameplayStatics.GetPlayerController` 0)))

(event `self.ReceiveTick`
  (params (DeltaSeconds :type "Float (single-precision)")))

(event `Key|E`
  (params (Key :type "Key Structure" :default "AnyKey"))
  (:`Pressed`
    (if (== (`self.Tutorial Level`) 1)
      (set `self.Tutorial Level` 2)
      (`SceneComponent.SetVisibility` (`self.Tutorial1`) false false)
      (`SceneComponent.SetVisibility` (`self.Tutorial2`) true false))))

(fn `UserConstructionScript`)