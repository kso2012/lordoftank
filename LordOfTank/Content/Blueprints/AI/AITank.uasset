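; AITank is an AI tank Blueprint that spawns a LOTDrone on BeginPlay and registers itself with the single-game mode.
; The drone spawns at the DronePosition component's relative transform, then tank and drone are passed to Single_GameMode's SavePlayerInfo as player 0.
; Tick only prints the game mode's PlayerCount as debug output, and the overlap event and construction script are empty.
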(event `self.ReceiveBeginPlay`
  (bind _returnvalue (`|SpawnActorFromClass` "/Script/LordOfTank.LOTDrone" (`SceneComponent.GetRelativeTransform` (`self.Drone Position`)) "Undefined" "OverrideRootScale"))
  (bind _assingle_game_mode (cast `/Game/Blueprints/Single_GameMode` (`GameplayStatics.GetGameMode`)))
  (`LordOfTankGameModeBase.SavePlayerInfo` _assingle_game_mode self _returnvalue 0))

(event `self.ReceiveTick`
  (params (DeltaSeconds :type "Float (single-precision)"))
  (`KismetSystemLibrary.PrintString` (`KismetStringLibrary.Conv_IntToString` (`LordOfTankGameModeBase.PlayerCount` (stale `self.ReceiveBeginPlay` _assingle_game_mode)))))

(fn `UserConstructionScript`)