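; AI controller that walks a Cube_Blueprint pawn along a chain of linked path nodes.
; On BeginPlay it caches the controlled pawn and moves to that pawn's DesireNode.
; Tick polls the move status and, whenever it differs from DesiredStatus, advances DesireNode to its NextNode and issues a new MoveToActor.
; A disconnected copy of the same logic for an AITank pawn never runs.
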(event `self.ReceiveBeginPlay`
  (bind _ascube_blueprint (cast `/Game/Blueprints/AI/Cube_Blueprint` (`self.K2_GetPawn`)))
  (bind _output_get (set `self.Stored Cube` _ascube_blueprint))
  (`self.MoveToActor` (`/Game/Blueprints/AI/Cube_Blueprint.Desire Node` _output_get) 15.0))

(event `self.ReceiveTick`
  (params (DeltaSeconds :type "Float (single-precision)"))
  (bind _stored_cube (`self.Stored Cube`))
  (if (!= (`self.GetMoveStatus`) (`self.desiredStatus`))
    (bind _output_get (set `/Game/Blueprints/AI/Cube_Blueprint.Desire Node` (`/Game/Blueprints/AI/Path.Next Node` (`/Game/Blueprints/AI/Cube_Blueprint.Desire Node` _stored_cube)) _stored_cube))
    (`self.MoveToActor` _output_get 15.0)))

(fn `UserConstructionScript`)